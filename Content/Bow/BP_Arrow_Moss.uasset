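; BP_Arrow_Moss is an arrow actor that plants a BP_Moss patch on the surface below where it hits.
; When its Cylinder component hits, it line-traces up to 5000 units straight down on Visibility, with debug drawing enabled.
; On a blocking hit it spawns the moss just above the impact point, matches the hit actor's rotation rather than the surface normal, then destroys itself.
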(event OnComponentHit(Cylinder)
  (params (HitComponent :type Primitive%20Component%20Object%20Reference) (OtherActor :type Actor%20Object%20Reference) (OtherComp :type Primitive%20Component%20Object%20Reference) (NormalImpulse :type Vector :default "0, 0, 0") (Hit :type Hit%20Result%20Structure%20%28by%20ref%29))
  (bind _returnvalue (Transformation|GetActorLocation))
  (bind _outhit (Collision|LineTraceByChannel (+ _returnvalue (* (Math|Vector|GetUpVector "0, 0, 0") -2)) (- _returnvalue "0.000000,0.000000,5000.000000") "TraceTypeQuery1" false 0 "ForDuration"))
  (if (.bBlockingHit (Collision|BreakHitResult _outhit))
    (bind _returnvalue_2 (Game|SpawnActorfromClass "/Game/Bow/BP_Moss.BP_Moss_C" (Math|Conversions|ToTransform(Vector) (+ (.ImpactPoint (Collision|BreakHitResult _outhit)) "0.000000,0.000000,1.000000")) "Undefined" "MultiplyWithRoot" 0 0))
    (Transformation|SetActorRotation _returnvalue_2 (Transformation|GetActorRotation (.HitActor (Collision|BreakHitResult _outhit))))
    (Actor|DestroyActor)))

(event EventBeginPlay
  (|CallParentFunction) ; This node is disabled and will not be called.\nDrag off pins to build functionality.
)

(event Collision|EventActorBeginOverlap
  (params (OtherActor :type Actor%20Object%20Reference))
  (|CallParentFunction OtherActor) ; This node is disabled and will not be called.\nDrag off pins to build functionality.
)

(event EventTick
  (params (DeltaSeconds :type Float%20%28single-precision%29))
  (|CallParentFunction DeltaSeconds) ; This node is disabled and will not be called.\nDrag off pins to build functionality.
)

(fn ConstructionScript
  (|CallParentFunction))