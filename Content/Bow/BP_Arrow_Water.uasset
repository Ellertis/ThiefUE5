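; BP_Arrow_Water is a water arrow for the bow that extinguishes objects it hits.
; When its Cylinder component hits an actor, it prints that actor's name, sends TurnOffMessage if the actor implements BPI_Extinghuishable, then destroys itself on any hit.
; On BeginPlay it runs the parent logic and starts a five-second timer, apparently to self-destruct if nothing is hit.
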(event OnComponentHit(Cylinder)
  (params (HitComponent :type Primitive%20Component%20Object%20Reference) (OtherActor :type Actor%20Object%20Reference) (OtherComp :type Primitive%20Component%20Object%20Reference) (NormalImpulse :type Vector :default "0, 0, 0") (Hit :type Hit%20Result%20Structure%20%28by%20ref%29))
  (Development|PrintString (Utilities|GetDisplayName OtherActor))
  (if (Utilities|DoesObjectImplementInterface OtherActor "/Game/Bow/BPI_Extinghuishable.BPI_Extinghuishable_C")
    (Class|BPIExtinghuishable|TurnOff(Message) OtherActor))
  (Actor|DestroyActor))

(event Custom|DestroySelfAfterDelay
  (Actor|DestroyActor))

(event EventBeginPlay
  (|CallParentFunction)
  (Utilities|Time|SetTimerbyEvent (EventDispatchers|CreateEvent :!event Custom|DestroySelfAfterDelay) 5.0))

(event Collision|EventActorBeginOverlap
  (params (OtherActor :type Actor%20Object%20Reference))
  (|CallParentFunction OtherActor) ; This node is disabled and will not be called.\nDrag off pins to build functionality.
)

(event EventTick
  (params (DeltaSeconds :type Float%20%28single-precision%29))
  (|CallParentFunction DeltaSeconds) ; This node is disabled and will not be called.\nDrag off pins to build functionality.
)

(fn ConstructionScript
  (|CallParentFunction))