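; BP_Bow is a first-person bow actor with Enhanced Input draw, release and cancel actions.
; Holding draw builds charge over time, and reaching the maximum triggers a one-time camera FOV zoom through a reversible Timeline.
; Releasing checks charge against a threshold but only prints the result, as the arrow-spawning code is unconnected.
; Cancelling stores the player's forward vector as aim direction, and both release and cancel reset charge and zoom.
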(event Custom|SetBowAimDirection
  (Variables|Default|SetBowAimDirection (Transformation|GetActorForwardVector (Variables|Default|GetPlayerRef))))

(event Custom|ToggleZoom
  (if (Variables|Default|GetZooming)
    (Variables|Default|SetZooming false)
    (bind _zoom (Timeline|Timeline_1 Reverse)
      (:Update
        (Camera|SetFieldOfView (Variables|/Game/FirstPerson/Blueprints/BP_FirstPersonCharacter.BP_FirstPersonCharacter_C|GetFirstPersonCamera (Variables|Default|GetPlayerRef)) (Math|Float|Lerp (Variables|Default|GetDefaultFOV) (Variables|Default|GetZoomFOV) _zoom))))
    (else
      (Variables|Default|SetZooming true)
      (Timeline|Timeline_1 PlayFromStart))))

(event Input|EnhancedActionEvents|EnhancedInputActionIA_DrawArrow
  (params (ActionValue :type Boolean) (ElapsedSeconds :type Float%20%28double-precision%29) (TriggeredSeconds :type Float%20%28double-precision%29) (InputAction :type Input%20Action%20Object%20Reference :default "/Game/FirstPerson/Input/Actions/IA_DrawArrow.IA_DrawArrow"))
  (:Triggered
    (if (Variables|Default|GetCharging)
      ;[1 1 1] Draw
      (bind _output_get (Variables|Default|SetCharge (+ (Variables|Default|GetCharge) (* (Utilities|Time|GetWorldDeltaSeconds) (Variables|Default|GetChargeSpeed)))))
      (Development|PrintString (Utilities|String|Append "Holding" (Utilities|String|ToString(Float) _output_get)))
      (if (>= (Variables|Default|GetCharge) (Variables|Default|GetMaxCharge))
        (Utilities|FlowControl|DoOnce false :!label _label
          (:Completed
            (CallFunction|ToggleZoom)
            (Variables|Default|SetZoomed true)
            (Development|PrintString "Zoom"))))))
  (:Started
    (Variables|Default|SetCharging true))
  (:Completed
    (if (CallFunction|EnoughChargetoShoot?)
      (Development|PrintString "Shoot")
      (else
        (Development|PrintString "Not Enough Charge")))
    (Variables|Default|SetCharge 0.0)
    (Variables|Default|SetCharging false)
    (if (Variables|Default|GetZoomed)
      (CallFunction|ToggleZoom)
      (Variables|Default|SetZoomed false)
      (goto _label Reset))))

(event Input|EnhancedActionEvents|EnhancedInputActionIA_CancelDrawArrow
  (params (ActionValue :type Boolean) (ElapsedSeconds :type Float%20%28double-precision%29) (TriggeredSeconds :type Float%20%28double-precision%29) (InputAction :type Input%20Action%20Object%20Reference :default "/Game/FirstPerson/Input/Actions/IA_CancelDrawArrow.IA_CancelDrawArrow"))
  (:Triggered
    (if (Variables|Default|GetCharging)
      (CallFunction|SetBowAimDirection)
      (Variables|Default|SetCharging false)
      (bind _output_get (Variables|Default|SetCharge 0.0))
      (Development|PrintString (Utilities|String|Append (Utilities|String|ToString(Float) _output_get) "Stopped Holding"))
      (if (Variables|Default|GetZoomed)
        (CallFunction|ToggleZoom)
        (Variables|Default|SetZoomed false)
        (Utilities|FlowControl|DoOnce false) ; enters at Reset
      ))))

(event EventBeginPlay
  (bind _returnvalue (Game|GetPlayerController 0))
  (Utilities|FlowControl|Sequence
    (:then_0
      (Input|EnableInput _returnvalue)
      (Input|AddMappingContext (PlayerController|LocalPlayerSubsystems|GetEnhancedInputLocalPlayerSubsystem _returnvalue) "/Game/FirstPerson/Input/IMC_Bow.IMC_Bow" 0 "(bIgnoreAllPressedKeysUntilRelease=True,bForceImmediately=False)"))
    (:then_1
      (bind _returnvalue_2 (Actor|GetActorOfClass "/Game/FirstPerson/Blueprints/BP_FirstPersonCharacter.BP_FirstPersonCharacter_C"))
      (bind _output_get (Variables|Default|SetPlayerRef _returnvalue_2))
      (Variables|Default|SetDefaultFOV (Variables|/Script/Engine.CameraComponent|GetFieldOfView (Variables|/Game/FirstPerson/Blueprints/BP_FirstPersonCharacter.BP_FirstPersonCharacter_C|GetFirstPersonCamera _output_get))))))

(event Collision|EventActorBeginOverlap
  (params (OtherActor :type Actor%20Object%20Reference)))

(event EventTick
  (params (DeltaSeconds :type Float%20%28single-precision%29)))

(fn ConstructionScript)

(fn EnoughChargetoShoot?
  (if (>= (Variables|Default|GetCharge) (Variables|Default|GetShotThreshold))
    (return true)
    (else
      (return false))))