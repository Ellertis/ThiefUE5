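; Rope arrow that, on hitting a wooden wall, becomes a climbable rope for the first-person character; any other hit destroys it.
; The first hit stops physics, then a downward trace sets the cable's end and length and sizes the capsule to span the drop.
; Interact inside the capsule calls the character's climb function, as does leaving it while climbing.
; The trace still draws debug lines, and an unconnected surface-type check never runs.
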(event OnComponentHit(Cylinder)
  (params (HitComponent :type Primitive%20Component%20Object%20Reference) (OtherActor :type Actor%20Object%20Reference) (OtherComp :type Primitive%20Component%20Object%20Reference) (NormalImpulse :type Vector :default "0, 0, 0") (Hit :type Hit%20Result%20Structure%20%28by%20ref%29))
  (bind _returnvalue (Transformation|GetActorLocation))
  (bind _returnvalue_2 (Transformation|GetActorLocation))
  (bind _cable (Variables|Default|GetCable))
  (bind _capsule (Variables|Default|GetCapsule))
  (Utilities|FlowControl|DoOnce false
    (:Completed
      (Physics|SetSimulatePhysics (Variables|Default|GetCylinder) false)
      (if (== (Utilities|GetClass OtherActor) "/Game/BP_Wall_Wood.BP_Wall_Wood_C")
        (bind _outhit (Collision|LineTraceByChannel (+ _returnvalue (* (Math|Vector|GetUpVector "0, 0, 0") -25)) (- _returnvalue "0.000000,0.000000,5000.000000") "TraceTypeQuery1" false 0 "ForDuration"))
        (Variables|/Script/CableComponent.CableComponent|SetEndLocation _cable (.ImpactPoint (Collision|BreakHitResult _outhit)))
        (Variables|/Script/CableComponent.CableComponent|SetCableLength _cable (Math|Vector|Distance(Vector) (.ImpactPoint (Collision|BreakHitResult _outhit)) _returnvalue_2))
        (Components|Capsule|SetCapsuleHalfHeight _capsule (* (Math|Vector|Distance(Vector) (.ImpactPoint (Collision|BreakHitResult _outhit)) _returnvalue_2) 0.5) false)
        (Transformation|SetWorldLocationAndRotation _capsule (+ (.ImpactPoint (Collision|BreakHitResult _outhit)) (Math|Vector|MakeVector 0.0 0.0 (* (.z (- _returnvalue_2 (.ImpactPoint (Collision|BreakHitResult _outhit)))) 0.5))) (Math|Rotator|MakeRotfromZX (.ImpactNormal (Collision|BreakHitResult _outhit)) (Math|Vector|GetUpVector "0, 0, 0")) false false)
        (Collision|SetCollisionEnabled (Variables|Default|GetCylinder) "NoCollision")
        (else
          (Actor|DestroyActor))))))

(event OnComponentBeginOverlap(Capsule)
  (params (OverlappedComponent :type Primitive%20Component%20Object%20Reference) (OtherActor :type Actor%20Object%20Reference) (OtherComp :type Primitive%20Component%20Object%20Reference) (OtherBodyIndex :type Integer) (bFromSweep :type Boolean) (SweepResult :type Hit%20Result%20Structure%20%28by%20ref%29))
  (if (== OtherActor (Variables|Default|GetAs%20BP%20First%20Person%20Character))
    (Variables|Default|SetPlayerOverlap true)))

(event OnComponentEndOverlap(Capsule)
  (params (OverlappedComponent :type Primitive%20Component%20Object%20Reference) (OtherActor :type Actor%20Object%20Reference) (OtherComp :type Primitive%20Component%20Object%20Reference) (OtherBodyIndex :type Integer))
  (bind _as_bp_first_person_character (Variables|Default|GetAs%20BP%20First%20Person%20Character))
  (if (== OtherActor (Variables|Default|GetAs%20BP%20First%20Person%20Character))
    (Variables|Default|SetPlayerOverlap false)
    (if (Variables|/Game/FirstPerson/Blueprints/BP_FirstPersonCharacter.BP_FirstPersonCharacter_C|GetClimbing _as_bp_first_person_character)
      (Default|ClimbMyAss _as_bp_first_person_character))))

(event EventBeginPlay
  (|CallParentFunction)
  (bind _asbp_first_person_character (Utilities|Casting|CastToBP_FirstPersonCharacter (Game|GetPlayerCharacter 0)))
  (Variables|Default|SetAs%20BP%20First%20Person%20Character _asbp_first_person_character))

(event Collision|EventActorBeginOverlap
  (params (OtherActor :type Actor%20Object%20Reference))
  (|CallParentFunction OtherActor) ; This node is disabled and will not be called.\nDrag off pins to build functionality.
)

(event EventTick
  (params (DeltaSeconds :type Float%20%28single-precision%29))
  (|CallParentFunction DeltaSeconds))

(event EventInteract
  (if (Variables|Default|GetPlayerOverlap)
    (Default|ClimbMyAss (Variables|Default|GetAs%20BP%20First%20Person%20Character))))

(fn ConstructionScript
  (|CallParentFunction))