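; BP_Torch is a torch that can be switched on and off, driving a PointLight_ShadowDetection child actor as its light.
; BeginPlay caches that child actor, and both it and the construction script set the light's intensity from the Lit flag.
; Turnon and TurnOff change intensity and keep both actors' Lit flags in step; only Turnon clears SomeoneOccupied and plays a switch sound.
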(event EventBeginPlay
  (bind _aspoint_light_shadow_detection (Utilities|Casting|CastToPointLight_ShadowDetection (Variables|/Script/Engine.ChildActorComponent|GetChildActor (Variables|Default|GetChildActor))))
  (Variables|Default|SetAs%20Point%20Light%20Shadow%20Detection _aspoint_light_shadow_detection)
  (if (Variables|Default|GetLit)
    (Rendering|Components|Light|SetIntensity (Variables|/Game/Environment/PointLight_ShadowDetection.PointLight_ShadowDetection_C|GetPointLight (Variables|Default|GetAs%20Point%20Light%20Shadow%20Detection)) 5e+03)
    (else
      (Rendering|Components|Light|SetIntensity (Variables|/Game/Environment/PointLight_ShadowDetection.PointLight_ShadowDetection_C|GetPointLight (Variables|Default|GetAs%20Point%20Light%20Shadow%20Detection)) 0.0))))

(event Collision|EventActorBeginOverlap
  (params (OtherActor :type Actor%20Object%20Reference)))

(event EventTick
  (params (DeltaSeconds :type Float%20%28single-precision%29)))

(event EventTurnon
  (if (not (Variables|Default|GetLit))
    (Rendering|Components|Light|SetIntensity (Variables|/Game/Environment/PointLight_ShadowDetection.PointLight_ShadowDetection_C|GetPointLight (Variables|Default|GetAs%20Point%20Light%20Shadow%20Detection)) 5e+03)
    (Variables|/Game/Environment/PointLight_ShadowDetection.PointLight_ShadowDetection_C|SetLit (Variables|Default|GetAs%20Point%20Light%20Shadow%20Detection) true)
    (Variables|Default|SetSomeoneOccupied false)
    (Variables|Default|SetLit true)
    (Audio|PlaySoundatLocation "/Game/Sounds/Switch.Switch" (Transformation|GetActorLocation) "0, 0, 0" 1.0 1.0 0.0 0 0 0 0)))

(event EventTurnOff
  (if (Variables|Default|GetLit)
    (Rendering|Components|Light|SetIntensity (Variables|/Game/Environment/PointLight_ShadowDetection.PointLight_ShadowDetection_C|GetPointLight (Variables|Default|GetAs%20Point%20Light%20Shadow%20Detection)) 0.0)
    (Variables|/Game/Environment/PointLight_ShadowDetection.PointLight_ShadowDetection_C|SetLit (Variables|Default|GetAs%20Point%20Light%20Shadow%20Detection) false)
    (Variables|Default|SetLit false)))

(fn ConstructionScript
  (bind _as_point_light_shadow_detection (Variables|Default|GetAs%20Point%20Light%20Shadow%20Detection))
  (bind _pointlight (Variables|/Game/Environment/PointLight_ShadowDetection.PointLight_ShadowDetection_C|GetPointLight _as_point_light_shadow_detection))
  (if (Variables|Default|GetLit)
    (Rendering|Components|Light|SetIntensity _pointlight 5e+03)
    (else
      (Rendering|Components|Light|SetIntensity _pointlight 0.0))))