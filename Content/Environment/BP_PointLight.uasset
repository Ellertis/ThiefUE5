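; Point light actor that checks the player within its radius and writes a PlayerVisible flag to the Singleton game instance.
; A sphere sized to the light's attenuation radius pauses and unpauses a looping trace timer as the player leaves and enters.
; Visibility traces run from the light to the capsule's top and bottom, with debug drawing.
; The flag is true when either trace's hit actor is not the player, including no hit.
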(event OnComponentBeginOverlap(Sphere)
  (params (OverlappedComponent :type Primitive%20Component%20Object%20Reference) (OtherActor :type Actor%20Object%20Reference) (OtherComp :type Primitive%20Component%20Object%20Reference) (OtherBodyIndex :type Integer) (bFromSweep :type Boolean) (SweepResult :type Hit%20Result%20Structure%20%28by%20ref%29))
  (if (== OtherActor (Game|GetPlayerCharacter 0))
    (Variables|Default|SetPlayerInside true)
    (Utilities|Time|UnpauseTimerbyHandle (Variables|Default|GetTracePlayerTimer))))

(event OnComponentEndOverlap(Sphere)
  (params (OverlappedComponent :type Primitive%20Component%20Object%20Reference) (OtherActor :type Actor%20Object%20Reference) (OtherComp :type Primitive%20Component%20Object%20Reference) (OtherBodyIndex :type Integer))
  (if (== OtherActor (Game|GetPlayerCharacter 0))
    (Variables|Default|SetPlayerInside false)
    (Utilities|Time|PauseTimerbyHandle (Variables|Default|GetTracePlayerTimer))))

(event Custom|TracePlayer
  (bind _returnvalue (Game|GetPlayerCharacter 0))
  (bind _as_singleton (Variables|Default|GetAs%20Singleton))
  (bind _returnvalue_2 (Transformation|GetActorLocation _returnvalue))
  (bind _capsulecomponent (Variables|/Script/Engine.Character|GetCapsuleComponent _returnvalue))
  (bind _capsulehalfheight (Variables|/Script/Engine.CapsuleComponent|GetCapsuleHalfHeight _capsulecomponent))
  (bind _visible (CallFunction|LineTracetoPlayer (- _returnvalue_2 (Math|Vector|MakeVector 0.0 0.0 _capsulehalfheight))))
  (bind _visible_2 (CallFunction|LineTracetoPlayer (+ _returnvalue_2 (Math|Vector|MakeVector 0.0 0.0 _capsulehalfheight))))
  (if (or _visible_2 _visible)
    (bind _output_get (Variables|Default|SetPlayerVisible true))
    (Variables|/Game/Singleton.Singleton_C|SetPlayerVisible _as_singleton _output_get)
    (else
      (bind _output_get_2 (Variables|Default|SetPlayerVisible false))
      (Variables|/Game/Singleton.Singleton_C|SetPlayerVisible _as_singleton _output_get_2))))

(event EventBeginPlay
  (bind _returnvalue (Utilities|Time|SetTimerbyEvent (EventDispatchers|CreateEvent :!event Custom|TracePlayer) 0.1 true))
  (bind _output_get (Variables|Default|SetTracePlayerTimer _returnvalue))
  (Utilities|Time|PauseTimerbyHandle _output_get)
  (bind _assingleton (Utilities|Casting|CastToSingleton (Game|GetGameInstance)))
  (Variables|Default|SetAs%20Singleton _assingleton))

(event Collision|EventActorBeginOverlap
  (params (OtherActor :type Actor%20Object%20Reference)))

(event EventTick
  (params (DeltaSeconds :type Float%20%28single-precision%29))
  (if (Variables|Default|GetPlayerInside)
    _))

(fn ConstructionScript
  (Components|Sphere|SetSphereRadius (Variables|Default|GetSphere) (Variables|/Script/Engine.LocalLightComponent|GetAttenuationRadius (Variables|Default|GetPointLight)) true))

(fn LineTracetoPlayer
  (params (Location :type Vector))
  (bind _outhit (Collision|LineTraceByChannel (Transformation|GetWorldLocation (Variables|Default|GetPointLight)) Location "TraceTypeQuery1" false 0 "ForDuration"))
  (return (not (== (.HitActor (Collision|BreakHitResult _outhit)) (Game|GetPlayerCharacter 0)))))