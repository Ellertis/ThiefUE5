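; BP_Fast_Poisson scatters static mesh instances around itself with Poisson-disc-style rejection sampling, in both the construction script and BeginPlay.
; It grows a HISM instance list up to SearchDepth, sampling random points between Radius1 and Radius2 from the actor's location.
; CheckNeighbours sphere-traces at Radius1, triggering limited retries when it hits any HISM component.
; The seeded stream is set, but RandomFloat calls do not use it.
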(event EventBeginPlay
  (bind _returnvalue (Math|Random|RandomFloat))
  (bind _returnvalue_2 (Math|Random|RandomFloat))
  (bind _returnvalue_3 (Transformation|GetActorLocation))
  (bind _hism (Variables|Default|GetHISM))
  (bind _radius1 (Variables|Default|GetRadius1))
  (bind _radius2 (Variables|Default|GetRadius2))
  (bind _returnvalue_4 (Math|Float|MapRangeClamped _returnvalue 0.0 1.0 _radius1 _radius2))
  (bind _returnvalue_5 (* _returnvalue_2 3.6e+02))
  (bind _returnvalue_6 (Math|Vector|GetForwardVector (Math|Rotator|MakeRotator 0.0 0.0 _returnvalue_5)))
  (bind _returnvalue_7 (* _returnvalue_6 _returnvalue_4))
  (bind _returnvalue_8 (+ _returnvalue_3 _returnvalue_7))
  (Math|Random|SetRandomStreamSeed (Variables|Default|GetStream) (Variables|Default|GetSeed))
  (Components|InstancedStaticMesh|ClearInstances _hism)
  (Components|StaticMesh|SetStaticMesh _hism (Variables|Default|GetStaticMesh))
  (if (> (Variables|Default|GetSearchDepth) 0)
    (bind _returnvalue_9 (Components|InstancedStaticMesh|AddInstance (Variables|Default|GetHISM) (Math|Transform|MakeTransform "0, 0, 0" "0, 0, 0" "1.000000,1.000000,1.000000") true))
    (Utilities|Array|AddUnique (Variables|Default|GetSpawnedInstances) _returnvalue_9)
    (for (_ _array_index) (Variables|Default|GetSpawnedInstances)
      (if (< _array_index (Variables|Default|GetSearchDepth)) :!label _label
        (bind _collision (CallFunction|CheckNeighbours _returnvalue_8))
        (if _collision
          (bind _result (Math|Integer|IncrementInt (Variables|Default|GetInnerSearchDepthCount))
            (:%20%20
              (if (< _result (Variables|Default|GetInnerSearchDepth))
                (goto _label)
                (else
                  (Variables|Default|SetInnerSearchDepthCount 0)))))
          (else
            (bind _returnvalue_10 (Components|InstancedStaticMesh|AddInstance (Variables|Default|GetHISM) (Math|Transform|MakeTransform _returnvalue_8 "0, 0, 0" "1.000000,1.000000,1.000000") true))
            (Utilities|Array|AddUnique (Variables|Default|GetSpawnedInstances) _returnvalue_10)
            (Variables|Default|SetInnerSearchDepthCount 0)))
        (else
          (Variables|Default|SetInnerSearchDepthCount 0))))))

(fn ConstructionScript
  (bind _returnvalue (Math|Random|RandomFloat))
  (bind _returnvalue_2 (Math|Random|RandomFloat))
  (bind _returnvalue_3 (Transformation|GetActorLocation))
  (bind _hism (Variables|Default|GetHISM))
  (bind _radius1 (Variables|Default|GetRadius1))
  (bind _radius2 (Variables|Default|GetRadius2))
  (bind _returnvalue_4 (Math|Float|MapRangeClamped _returnvalue 0.0 1.0 _radius1 _radius2))
  (bind _returnvalue_5 (* _returnvalue_2 3.6e+02))
  (bind _returnvalue_6 (Math|Vector|GetForwardVector (Math|Rotator|MakeRotator 0.0 0.0 _returnvalue_5)))
  (bind _returnvalue_7 (* _returnvalue_6 _returnvalue_4))
  (bind _returnvalue_8 (+ _returnvalue_3 _returnvalue_7))
  (Math|Random|SetRandomStreamSeed (Variables|Default|GetStream) (Variables|Default|GetSeed))
  (Components|InstancedStaticMesh|ClearInstances _hism)
  (Components|StaticMesh|SetStaticMesh _hism (Variables|Default|GetStaticMesh))
  (if (> (Variables|Default|GetSearchDepth) 0)
    (bind _returnvalue_9 (Components|InstancedStaticMesh|AddInstance (Variables|Default|GetHISM) (Math|Transform|MakeTransform "0, 0, 0" "0, 0, 0" "1.000000,1.000000,1.000000") false))
    (Utilities|Array|AddUnique (Variables|Default|GetSpawnedInstances) _returnvalue_9)
    (for (_ _array_index) (Variables|Default|GetSpawnedInstances)
      (if (< _array_index (Variables|Default|GetSearchDepth)) :!label _label
        (bind _collision (CallFunction|CheckNeighbours _returnvalue_8))
        (if _collision
          (bind _result (Math|Integer|IncrementInt (Variables|Default|GetInnerSearchDepthCount))
            (:%20%20
              (if (< _result (Variables|Default|GetInnerSearchDepth))
                (goto _label)
                (else
                  (Variables|Default|SetInnerSearchDepthCount 0)))))
          (else
            (bind _returnvalue_10 (Components|InstancedStaticMesh|AddInstance (Variables|Default|GetHISM) (Math|Transform|MakeTransform _returnvalue_8 "0, 0, 0" "1.000000,1.000000,1.000000") false))
            (Utilities|Array|AddUnique (Variables|Default|GetSpawnedInstances) _returnvalue_10)
            (Variables|Default|SetInnerSearchDepthCount 0)))
        (else
          (Variables|Default|SetInnerSearchDepthCount 0))))))

(fn CheckNeighbours
  (params (MeshLoc :type Vector))
  (bind _outhits (Collision|MultiSphereTraceByChannel MeshLoc MeshLoc (Variables|Default|GetRadius1) "TraceTypeQuery1" false 0 "ForDuration" false "(R=1.000000,G=0.000000,B=0.000000,A=1.000000)" "(R=0.000000,G=1.000000,B=0.000000,A=1.000000)" 0.0))
  (for _array_element _outhits
    (if (== (Utilities|GetClass (.HitComponent (Collision|BreakHitResult _array_element))) "/Script/Engine.HierarchicalInstancedStaticMeshComponent")
      (return true)))
  (return false))