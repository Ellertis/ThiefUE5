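; BP_Door is an interactable door that highlights when focused and swings open or closed on interaction.
; Highlight stores the focus state and toggles custom depth rendering on the door mesh.
; Interact uses a FlipFlop to play or reverse a Timeline, which lerps the door's relative yaw.
; Overlap and hit handlers check for the player but take no action, and debug prints remain.
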(event OnComponentBeginOverlap(Door)
  (params (OverlappedComponent :type Primitive%20Component%20Object%20Reference) (OtherActor :type Actor%20Object%20Reference) (OtherComp :type Primitive%20Component%20Object%20Reference) (OtherBodyIndex :type Integer) (bFromSweep :type Boolean) (SweepResult :type Hit%20Result%20Structure%20%28by%20ref%29))
  (if (== (stale OnComponentHit(Door) OtherActor) (Game|GetPlayerCharacter 0))
    _))

(event OnComponentHit(Door)
  (params (HitComponent :type Primitive%20Component%20Object%20Reference) (OtherActor :type Actor%20Object%20Reference) (OtherComp :type Primitive%20Component%20Object%20Reference) (NormalImpulse :type Vector :default "0, 0, 0") (Hit :type Hit%20Result%20Structure%20%28by%20ref%29))
  (if (== OtherActor (Game|GetPlayerCharacter 0))
    _))

(event EventBeginPlay)

(event Collision|EventActorBeginOverlap
  (params (OtherActor :type Actor%20Object%20Reference)))

(event EventTick
  (params (DeltaSeconds :type Float%20%28single-precision%29)))

(event EventInteract
  (Development|PrintString "Door open")
  (Utilities|FlowControl|FlipFlop
    (:A
      (bind _newtrack_0 (Timeline|Timeline Play)
        (:Update
          (Transformation|SetRelativeRotation (Variables|Default|GetDoor) (Math|Rotator|MakeRotator 0.0 0.0 (Math|Float|Lerp 0.0 -1.2e+02 _newtrack_0)) false false))))
    (:B
      (Timeline|Timeline Reverse))))

(event EventHighlight
  (params (True/False :type Boolean))
  (bind _door (Variables|Default|GetDoor))
  (bind _output_get (Variables|Default|SetFocused True/False))
  (if _output_get
    (Development|PrintString "Focus")
    (Rendering|SetRenderCustomDepth _door true)
    (else
      (Development|PrintString "Unfocus")
      (Rendering|SetRenderCustomDepth _door false))))

(fn ConstructionScript)