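; BP_Enemy_Melee is a melee enemy character that fights with a sword and signals when attack, equip and unequip actions finish.
; Attack plays a random montage from a list, while equip and unequip play over-the-shoulder montages guarded by the WieldingWeapon flag.
; Montage notifies time spawning the sword onto the hand socket and destroying it.
; SetMovementSpeed maps idle, walking, running and fighting states to walk speed.
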(event EventBeginPlay
  (|CallParentFunction) ; This node is disabled and will not be called.\nDrag off pins to build functionality.
)

(event EventEquipWeapon
  (if (not (Variables|Default|GetWieldingWeapon))
    (bind _notifyname (Animation|Montage|PlayMontage (Variables|Character|GetMesh) "/Game/Characters/Mannequins/Animations/Manny/Montage_UnarmedEquipOverShoulder_UE.Montage_UnarmedEquipOverShoulder_UE")
      (:OnCompleted
        (Default|CallOnWeaponEquipped))
      (:OnNotifyBegin
        (switch name _notifyname
          (:CreateWeapon
            (bind _returnvalue (Game|SpawnActorfromClass "/Game/Enemy/BP_Weapon_Sword.BP_Weapon_Sword_C" (Transformation|GetActorTransform) "Undefined" "MultiplyWithRoot" 0 0))
            (Variables|Default|SetWeaponActor _returnvalue)
            (bind _returnvalue_2 (Transformation|AttachComponentToComponent _returnvalue (Variables|Character|GetMesh) "hand_r_sword_socket" "SnapToTarget" "SnapToTarget" "KeepRelative" true))
            (Variables|Default|SetWieldingWeapon _returnvalue_2)))))))

(event EventUnequipWeapon
  (if (Variables|Default|GetWieldingWeapon)
    (bind _notifyname (Animation|Montage|PlayMontage (Variables|Character|GetMesh) "/Game/Characters/Mannequins/Animations/Manny/Montage_StandingDisarmOverShoulder_UE.Montage_StandingDisarmOverShoulder_UE")
      (:OnCompleted
        (Default|CallOnWeaponUnequipped))
      (:OnNotifyBegin
        (switch name _notifyname
          (:DeleteWeapon
            (Actor|DestroyActor (Variables|Default|GetWeaponActor))
            (Variables|Default|SetWieldingWeapon false)))))))

(event Collision|EventActorBeginOverlap
  (params (OtherActor :type Actor%20Object%20Reference)))

(event EventTick
  (params (DeltaSeconds :type Float%20%28single-precision%29)))

(event EventAttack
  (Animation|Montage|PlayMontage (Variables|Character|GetMesh) (.OutItem (Utilities|Array|Random (Variables|Default|GetAttackMontageList)))
    (:OnCompleted
      (Default|CallOnAttackEnd))))

(fn ConstructionScript
  (|CallParentFunction))

(fn SetMovementSpeed
  (params (Speed :type E_MovementSpeed%20Enum :default "NewEnumerator0"))
  (bind _output_get (Variables|/Script/Engine.CharacterMovementComponent|SetMaxWalkSpeed (Variables|Character|GetCharacterMovement) (Utilities|Select :Index Speed :NewEnumerator0 0.0 :NewEnumerator1 2e+02 :NewEnumerator2 4e+02 :NewEnumerator3 1.5e+02)))
  (return _output_get))