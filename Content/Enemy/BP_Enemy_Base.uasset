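; Base enemy character that delegates health, damage, healing and death to a damage system component and exposes patrol route, combat ranges and speed presets.
; Damage events halt movement, freeze the AI controller's state and play a random reaction montage, then set it attacking the damage causer.
; Death turns on mesh physics and stops AI logic.
; A torch-lighting montage fires events on notify and completion.
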(event Custom|OnDeath
  (bind _aicontroller (Variables|Default|GetAIController))
  (bind _mesh (Variables|Character|GetMesh))
  (Physics|SetSimulatePhysics _mesh true)
  (Collision|SetCollisionEnabled _mesh "QueryAndPhysics")
  (AI|Logic|StopLogic (Variables|/Script/AIModule.AIController|GetBrainComponent _aicontroller) "")
  (Default|SetStateasDead _aicontroller))

(event Custom|OnDamageResponse
  (params (DamageResponse :type E_DamageResponse%20Enum :default "NewEnumerator0") (DamageCauser :type Actor%20Object%20Reference))
  (bind _aicontroller (Variables|Default|GetAIController))
  (Components|Movement|StopMovementImmediately (Variables|Character|GetCharacterMovement))
  (Default|SetStateasFrozen _aicontroller)
  (Animation|Montage|PlayMontage (Variables|Character|GetMesh) (.OutItem (Utilities|Array|Random (Variables|Default|GetDamageReaction)))
    (:OnCompleted
      _)
    (:OnInterrupted
      _))
  (Default|SetStateasAttacking _aicontroller DamageCauser true))

(event EventBeginPlay
  (bind _bpc_damagesystem (Variables|Default|GetBPC_DamageSystem))
  (bind _asaic_enemy_base (Utilities|Casting|CastToAIC_Enemy_Base (AI|GetAIController self)))
  (Variables|Default|SetAIController _asaic_enemy_base)
  (EventDispatchers|AssignOnDeath _bpc_damagesystem (EventDispatchers|CreateEvent :!event Custom|OnDeath))
  (EventDispatchers|AssignOnDamageResponse _bpc_damagesystem (EventDispatchers|CreateEvent :!event Custom|OnDamageResponse)))

(event EventLightTorch
  (bind _notifyname (Animation|Montage|PlayMontage (Variables|Character|GetMesh) "/Game/Characters/Mannequins/Animations/Manny/Montage_PullingLever.Montage_PullingLever")
    (:OnCompleted
      (Default|CallOnTorchLitEnd))
    (:OnNotifyBegin
      (switch name _notifyname
        (:TorchLit
          (Default|CallTorchLit))))))

(fn ConstructionScript)

(fn GetCurrentHealth
  (return (Variables|/Game/DamageSystem/BPC_DamageSystem.BPC_DamageSystem_C|GetHealth (Variables|Default|GetBPC_DamageSystem))))

(fn GetIdealRange
  (return 1.5e+02 3e+02))

(fn GetMaxHealth
  (return (Variables|/Game/DamageSystem/BPC_DamageSystem.BPC_DamageSystem_C|GetMaxHealth (Variables|Default|GetBPC_DamageSystem))))

(fn GetPatrolRoute
  (return (Variables|Default|GetPatrolRoute)))

(fn Heal
  (params (Amount :type Float%20%28double-precision%29))
  (bind _newhealth (Default|Heal (Variables|Default|GetBPC_DamageSystem) Amount))
  (return _newhealth))

(fn IsDead
  (return (Variables|/Game/DamageSystem/BPC_DamageSystem.BPC_DamageSystem_C|GetDead (Variables|Default|GetBPC_DamageSystem))))

(fn SetMovementSpeed
  (params (Speed :type E_MovementSpeed%20Enum :default "NewEnumerator0"))
  (bind _output_get (Variables|/Script/Engine.CharacterMovementComponent|SetMaxWalkSpeed (Variables|Character|GetCharacterMovement) (Utilities|Select :Index Speed :NewEnumerator0 0.0 :NewEnumerator1 2e+02 :NewEnumerator2 5e+02 :NewEnumerator3 1.5e+02)))
  (return _output_get))

(fn TakeDamage
  (params (DamageInfo :type S%20Damage%20Info%20Structure) (DamageCauser :type Actor%20Object%20Reference))
  (bind _wasdamaged (Default|TakeDamage (Variables|Default|GetBPC_DamageSystem) DamageInfo DamageCauser))
  (return _wasdamaged))