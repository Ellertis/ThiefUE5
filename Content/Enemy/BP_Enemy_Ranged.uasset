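; Ranged enemy character that fights with a bow, overriding movement speeds and ideal attack and defend range.
; Equip and unequip montages use notifies to spawn or destroy the bow, signalling completion.
; Attack chains draw and recoil montages: notifies spawn the arrow in hand, then detach and launch it toward the AI controller's target.
; Interrupting the draw, or the recoil before release, destroys the arrow.
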(event Custom|DestroyProjectile
  (bind _projectileactor (Variables|Default|GetProjectileActor))
  (Utilities|IsValid _projectileactor
    (:Is%20Valid
      (Actor|DestroyActor _projectileactor))))

(event EventBeginPlay
  (|CallParentFunction))

(event Collision|EventActorBeginOverlap
  (params (OtherActor :type Actor%20Object%20Reference)))

(event EventTick
  (params (DeltaSeconds :type Float%20%28single-precision%29)))

(event EventEquipWeapon
  (if (not (Variables|Default|GetWieldingWeapon))
    (bind _notifyname (Animation|Montage|PlayMontage (Variables|Character|GetMesh) "/Game/Characters/Mannequins/Animations/Manny/Ranged/Montage_StandingEquipBow_U.Montage_StandingEquipBow_U")
      (:OnCompleted
        (Default|CallOnWeaponEquipped))
      (:OnNotifyBegin
        (switch name _notifyname
          (:CreateWeapon
            (bind _returnvalue (Game|SpawnActorfromClass "/Game/Enemy/BP_Weapon_Bow.BP_Weapon_Bow_C" (Transformation|GetActorTransform) "Undefined" "MultiplyWithRoot" 0 0))
            (Variables|Default|SetWeaponActor _returnvalue)
            (bind _returnvalue_2 (Transformation|AttachComponentToComponent _returnvalue (Variables|Character|GetMesh) "hand_l_bow_socket" "SnapToTarget" "SnapToTarget" "KeepRelative" true))
            (Variables|Default|SetWieldingWeapon _returnvalue_2)))))))

(event EventUnequipWeapon
  (if (Variables|Default|GetWieldingWeapon)
    (bind _notifyname (Animation|Montage|PlayMontage (Variables|Character|GetMesh) "/Game/Characters/Mannequins/Animations/Manny/Ranged/Montage_StandingDisarmBow_UE.Montage_StandingDisarmBow_UE")
      (:OnCompleted
        (Default|CallOnWeaponUnequipped))
      (:OnNotifyBegin
        (switch name _notifyname
          (:DeleteWeapon
            (Actor|DestroyActor (Variables|Default|GetWeaponActor))
            (Variables|Default|SetWieldingWeapon false)))))))

(event EventAttack
  (bind _mesh (Variables|Character|GetMesh))
  (bind _notifyname (Animation|Montage|PlayMontage _mesh "/Game/Characters/Mannequins/Animations/Manny/Ranged/Montage_StandingDrawArrow_UE.Montage_StandingDrawArrow_UE")
    (:OnCompleted
      (bind _notifyname_2 (Animation|Montage|PlayMontage _mesh "/Game/Characters/Mannequins/Animations/Manny/Ranged/Montage_StandingAimRecoil_UE.Montage_StandingAimRecoil_UE")
        (:OnCompleted
          (Default|CallOnAttackEnd))
        (:OnInterrupted
          (if (not (Variables|Default|GetProjectileDetached))
            (CallFunction|DestroyProjectile)))
        (:OnNotifyBegin
          (switch name _notifyname_2
            (:Fire
              (Transformation|DetachFromActor (Variables|Default|GetProjectileActor) "KeepRelative" "KeepRelative" "KeepRelative")
              (Transformation|SetActorLocation (Variables|Default|GetProjectileActor) (+ (* (Transformation|GetActorForwardVector) 200) (Transformation|GetActorLocation)) false false)
              (Transformation|SetWorldRotation (Variables|/Script/Engine.Actor|GetRootComponent (Variables|Default|GetProjectileActor)) (Math|Rotator|FindLookatRotation (Transformation|GetWorldLocation (Variables|/Script/Engine.Actor|GetRootComponent (Variables|Default|GetProjectileActor))) (Transformation|GetActorLocation (Variables|/Game/Enemy/AI/AIC_Enemy_Base.AIC_Enemy_Base_C|GetAttack%20Target (Variables|Default|GetAIController)))) false false)
              (Default|LaunchArrow (Variables|Default|GetProjectileActor) self)
              (Variables|Default|SetProjectileDetached true))))))
    (:OnInterrupted
      (CallFunction|DestroyProjectile))
    (:OnNotifyBegin
      (switch name _notifyname
        (:Create%20Arrow
          (bind _returnvalue (Game|SpawnActorfromClass "/Game/Enemy/BP_Enemy_Arrow.BP_Enemy_Arrow_C" (Transformation|GetActorTransform) "Undefined" "MultiplyWithRoot" 0 0))
          (bind _output_get (Variables|Default|SetProjectileActor _returnvalue))
          (Transformation|AttachComponentToComponent _output_get (Variables|Character|GetMesh) "hand_l_arrow_socket" "SnapToTarget" "SnapToTarget" "KeepRelative" true)
          (Variables|Default|SetProjectileDetached false))))))

(fn ConstructionScript
  (|CallParentFunction))

(fn SetMovementSpeed
  (params (Speed :type E_MovementSpeed%20Enum :default "NewEnumerator0"))
  (bind _output_get (Variables|/Script/Engine.CharacterMovementComponent|SetMaxWalkSpeed (Variables|Character|GetCharacterMovement) (Utilities|Select :Index Speed :NewEnumerator0 0.0 :NewEnumerator1 2e+02 :NewEnumerator2 5e+02 :NewEnumerator3 1.5e+02)))
  (return _output_get))

(fn GetIdealRange
  (return 6e+02 6e+02))